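; PhoneCharacter_BP is an AI-controlled phone enemy with health, hit reactions and death.
; Damage not caused by the phone AI controller lowers health, updates the health widget and briefly pulses the "gethit" blackboard flag.
; At zero health it hides the bar and, once, increments the player's KillCount, stops AI logic, plays and freezes the death animation, and disables movement.
; An overlap volume shows the health widget only while the player is inside.
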(event `self.ReceiveAnyDamage`
  (params (Damage :type "Float (single-precision)") (DamageType :type "DamageType Object Reference") (InstigatedBy :type "Controller Object Reference") (DamageCauser :type "Actor Object Reference"))
  (bind _returnvalue (`AIBlueprintHelperLibrary.GetBlackboard` null))
  (bind _returnvalue_2 (`GameplayStatics.GetActorOfClass` "/Game/Phone_AI/PhoneAIController_BP.PhoneAIController_BP_C"))
  (if (not (== _returnvalue_2 DamageCauser))
    (bind _output_get (set `self.Health` (- (`self.Health`) Damage)))
    (set `/Game/Phone_AI/PhoneHealthWig.Health` _output_get (`self.PhoneHealth REF`))
    (if (<= _output_get 0.0)
      (`Widget.SetVisibility` (`self.PhoneHealth REF`) "Hidden")
      (`/Engine/EditorBlueprintResources/StandardMacros.DoOnce` false
        (:`Completed`
          (bind _asbp_third_person_character_child (cast `/Game/ThirdPerson/Blueprints/BP_ThirdPersonCharacter_Child` (`GameplayStatics.GetPlayerPawn` 0)))
          (`/Engine/EditorBlueprintResources/StandardMacros.IncrementInt` (`/Game/ThirdPerson/Blueprints/BP_ThirdPersonCharacter_Child.Kill Count` _asbp_third_person_character_child)
            (:`  `
              (`BrainComponent.StopLogic` (`AIController.BrainComponent` (`AIBlueprintHelperLibrary.GetAIController` self)) "Dead")
              (`SkeletalMeshComponent.PlayAnimation` (`self.Mesh`) "/Game/Phone_AI/mobileriged_Anim_Phaone_Bones_phoneDead.mobileriged_Anim_Phaone_Bones_phoneDead" false)
              (`KismetSystemLibrary.Delay` 0.8)
              (set `SkeletalMeshComponent.bPauseAnims` true (`self.Mesh`))
              (`CharacterMovementComponent.DisableMovement` (`self.CharacterMovement`))))))
      (else
        (bind _output_get_2 (set `self.isGetHit` true))
        (`BlackboardComponent.SetValueAsBool` _returnvalue "gethit" _output_get_2)
        (`KismetSystemLibrary.Delay` 0.4)
        (bind _output_get_3 (set `self.isGetHit` false))
        (`BlackboardComponent.SetValueAsBool` _returnvalue "gethit" _output_get_3)))))

(event `self.ReceiveBeginPlay`
  (bind _asphone_health_wig (cast `/Game/Phone_AI/PhoneHealthWig` (`WidgetComponent.GetUserWidgetObject` (`self.Widget`))))
  (set `self.PhoneHealth REF` _asphone_health_wig))

(event `self.healthIndication.OnComponentBeginOverlap`
  (params (OverlappedComponent :type "PrimitiveComponent Object Reference") (OtherActor :type "Actor Object Reference") (OtherComp :type "PrimitiveComponent Object Reference") (OtherBodyIndex :type Integer) (bFromSweep :type Boolean) (SweepResult :type "HitResult Structure (by ref)"))
  (cast `/Game/ThirdPerson/Blueprints/BP_ThirdPersonCharacter_Child` OtherActor)
  (`SceneComponent.SetVisibility` (`self.Widget`) true false))

(event `self.healthIndication.OnComponentEndOverlap`
  (params (OverlappedComponent :type "PrimitiveComponent Object Reference") (OtherActor :type "Actor Object Reference") (OtherComp :type "PrimitiveComponent Object Reference") (OtherBodyIndex :type Integer))
  (cast `/Game/ThirdPerson/Blueprints/BP_ThirdPersonCharacter_Child` OtherActor)
  (`SceneComponent.SetVisibility` (`self.Widget`) false false))

(fn `UserConstructionScript`)